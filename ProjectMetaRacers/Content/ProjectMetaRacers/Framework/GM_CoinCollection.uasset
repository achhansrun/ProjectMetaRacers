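; Game mode for a coin collection level in ProjectMetaRacers that quits the game once enough coins are collected.
; On BeginPlay it binds CoinCollected to only the first BP_Coin found, then sets TotalCoinCount from the final loop index over all coins, not the array length.
; Each CoinCollected event increments CoinCount and, on reaching TotalCoinCount, quits after a short delay.
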(event Custom|Coin%20Collected
  (Variables|Default|SetCoinCount (+ (Variables|Default|GetCoinCount) 1))
  (if (>= (Variables|Default|GetCoinCount) (Variables|Default|GetTotalCoinCount))
    (Utilities|FlowControl|Delay 0.45)
    (Game|QuitGame 0 "Quit" false)))

(event EventBeginPlay
  (|CallParentFunction)
  (bind _returnvalue (Actor|GetActorOfClass "/Game/GamePieces/Coin/BP_Coin.BP_Coin_C"))
  (EventDispatchers|BindEventtoCoinCollected _returnvalue (delegate Custom|Coin%20Collected))
  (bind _outactors (Actor|GetAllActorsOfClass "/Game/GamePieces/Coin/BP_Coin.BP_Coin_C"))
  (for (_ _array_index) _outactors
    _)
  (Variables|Default|SetTotalCoinCount _array_index))

(event EventTick
  (params (DeltaSeconds :type Float%20%28single-precision%29))
  (|CallParentFunction DeltaSeconds) ; This node is disabled and will not be called.\nDrag off pins to build functionality.
)

(fn ConstructionScript
  (|CallParentFunction))