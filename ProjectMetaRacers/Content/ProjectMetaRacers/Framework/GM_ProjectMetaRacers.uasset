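; Game mode for ProjectMetaRacers that runs a checkpoint race against a countdown timer.
; On BeginPlay it binds to the start line, every checkpoint and, inside that same loop, the finish line.
; The start line starts a minutes-and-seconds countdown, stepped by a one-second Delay on Tick, and checkpoints add seconds.
; Both crossing the finish line and running out of time quit the game.
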(event Custom|Finish%20Line
  (Game|QuitGame 0 "Quit" false))

(event Custom|Start%20Timer%20Event
  (bind _output_get (Variables|Default|SetTimer%20Started true)))

(event Custom|Checkpoint
  (Variables|Default|SetTimerSeconds (+ (Variables|Default|GetCheckpointAddTime) (Variables|Default|GetTimerSeconds))))

(event EventBeginPlay
  (bind _returnvalue (Actor|GetActorOfClass "/Game/GamePieces/StartLine/BP_StartLine.BP_StartLine_C"))
  (EventDispatchers|BindEventtoStartTimer _returnvalue (delegate Custom|Start%20Timer%20Event))
  (bind _outactors (Actor|GetAllActorsOfClass "/Game/GamePieces/BP_Checkpoint.BP_Checkpoint_C"))
  (for _array_element _outactors
    (bind _asbp_checkpoint (Utilities|Casting|CastToBP_Checkpoint _array_element))
    (EventDispatchers|BindEventtoCheckpoint _asbp_checkpoint (delegate Custom|Checkpoint))
    (bind _returnvalue_2 (Actor|GetActorOfClass "/Game/GamePieces/BP_FinishLine.BP_FinishLine_C"))
    (EventDispatchers|BindEventtoFinishLine _returnvalue_2 (delegate Custom|Finish%20Line))))

(event EventTick
  (params (DeltaSeconds :type Float%20%28single-precision%29))
  (if (stale Custom|Start%20Timer%20Event _output_get)
    (Utilities|FlowControl|Delay 1.0)
    (if (== (Variables|Default|GetTimerSeconds) 0)
      (if (== (Variables|Default|GetTimerMinutes) 0)
        (Game|QuitGame 0 "Quit" false)
        (else
          (Variables|Default|SetTimerSeconds 59)
          (Variables|Default|SetTimerMinutes (- (Variables|Default|GetTimerMinutes) 1))))
      (else
        (bind _output_get (Variables|Default|SetTimerSeconds (- (Variables|Default|GetTimerSeconds) 1)))
        (Development|PrintString (Utilities|String|ToString(Integer) _output_get))))))

(fn ConstructionScript)